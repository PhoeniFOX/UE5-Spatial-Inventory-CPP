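; BP_Knife is the knife item actor, which supplies its own item data, apparently for a grid-based inventory.
; GetDefaultItemObject constructs and initializes an ItemObject with a two-by-one footprint, normal and likely rotated icon materials, and BP_Knife as the item class.
; The event graph and construction script add no logic of their own.
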(fn `GetDefaultItemObject`
  (returns (ReturnValue :type "ItemObject Object Reference"))
  (bind _returnvalue (`|GenericCreateObject` "/Script/InventoryProjectCpp.ItemObject"))
  (`ItemObject.InitializeItemObject` _returnvalue 2 1 "/Game/Icons/MI_Icon_Knife.MI_Icon_Knife" "/Game/Icons/MI_Icon_Knife_R.MI_Icon_Knife_R" "BP_Knife_C")
  (return _returnvalue))

(fn `UserConstructionScript`
  (`parent.UserConstructionScript`))